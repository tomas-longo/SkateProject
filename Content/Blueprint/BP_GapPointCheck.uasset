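; BP_GapPointCheck is a gap scoring actor that awards RampPoints to a skater who jumps from one check volume and lands in the other, in either direction.
; Check1 and Check2 overlaps track presence and bind or unbind the skater's jump/fall and land events.
; Jump records the occupied volume, and land tests the opposite one, then clears the jump flags.
; A successful gap adds points through BP_SkaterPlayerState.
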(event OnComponentBeginOverlap(Check1)
  (params (OverlappedComponent :type Primitive%20Component%20Object%20Reference) (OtherActor :type Actor%20Object%20Reference) (OtherComp :type Primitive%20Component%20Object%20Reference) (OtherBodyIndex :type Integer) (bFromSweep :type Boolean) (SweepResult :type Hit%20Result%20Structure%20%28by%20ref%29))
  (bind _asbp_skater_character (Utilities|Casting|CastToBP_SkaterCharacter OtherActor))
  (Variables|Default|SetInsideCheck1 true)
  (bind _output_get (Variables|Default|SetSkaterCharacter _asbp_skater_character))
  (EventDispatchers|BindEventtoSkaterJumpFall _output_get (EventDispatchers|CreateEvent :!event Custom|OnSkaterJump))
  (EventDispatchers|BindEventtoSkaterLand (Variables|Default|GetSkaterCharacter) (EventDispatchers|CreateEvent :!event Custom|OnSkaterLand)))

(event OnComponentEndOverlap(Check1)
  (params (OverlappedComponent :type Primitive%20Component%20Object%20Reference) (OtherActor :type Actor%20Object%20Reference) (OtherComp :type Primitive%20Component%20Object%20Reference) (OtherBodyIndex :type Integer))
  (Utilities|Casting|CastToBP_SkaterCharacter OtherActor)
  (Variables|Default|SetInsideCheck1 false)
  (bind _skatercharacter (Variables|Default|GetSkaterCharacter)
    (:then
      (EventDispatchers|UnbindEventfromSkaterJumpFall _skatercharacter (EventDispatchers|CreateEvent :!event Custom|OnSkaterJump))
      (EventDispatchers|UnbindEventfromSkaterLand (Variables|Default|GetSkaterCharacter) (EventDispatchers|CreateEvent :!event Custom|OnSkaterLand)))
    (:else)))

(event OnComponentBeginOverlap(Check2)
  (params (OverlappedComponent :type Primitive%20Component%20Object%20Reference) (OtherActor :type Actor%20Object%20Reference) (OtherComp :type Primitive%20Component%20Object%20Reference) (OtherBodyIndex :type Integer) (bFromSweep :type Boolean) (SweepResult :type Hit%20Result%20Structure%20%28by%20ref%29))
  (bind _asbp_skater_character (Utilities|Casting|CastToBP_SkaterCharacter OtherActor))
  (Variables|Default|SetInsideCheck2 true)
  (bind _output_get (Variables|Default|SetSkaterCharacter _asbp_skater_character))
  (EventDispatchers|BindEventtoSkaterJumpFall _output_get (EventDispatchers|CreateEvent :!event Custom|OnSkaterJump))
  (EventDispatchers|BindEventtoSkaterLand (Variables|Default|GetSkaterCharacter) (EventDispatchers|CreateEvent :!event Custom|OnSkaterLand)))

(event OnComponentEndOverlap(Check2)
  (params (OverlappedComponent :type Primitive%20Component%20Object%20Reference) (OtherActor :type Actor%20Object%20Reference) (OtherComp :type Primitive%20Component%20Object%20Reference) (OtherBodyIndex :type Integer))
  (Utilities|Casting|CastToBP_SkaterCharacter OtherActor)
  (Variables|Default|SetInsideCheck2 false)
  (bind _skatercharacter (Variables|Default|GetSkaterCharacter)
    (:then
      (EventDispatchers|UnbindEventfromSkaterJumpFall _skatercharacter (EventDispatchers|CreateEvent :!event Custom|OnSkaterJump))
      (EventDispatchers|UnbindEventfromSkaterLand (Variables|Default|GetSkaterCharacter) (EventDispatchers|CreateEvent :!event Custom|OnSkaterLand)))
    (:else)))

(event Custom|OnSkaterJump
  (Variables|Default|SetJumpOnCheck1 (Variables|Default|GetInsideCheck1))
  (Variables|Default|SetJumpOnCheck2 (Variables|Default|GetInsideCheck2)))

(event Custom|OnSkaterLand
  (Utilities|FlowControl|Sequence
    (:then_0
      (if (or (and (Variables|Default|GetJumpOnCheck1) (Variables|Default|GetInsideCheck2)) (and (Variables|Default|GetJumpOnCheck2) (Variables|Default|GetInsideCheck1)))
        (CallFunction|RampJumped)))
    (:then_1
      (Variables|Default|SetJumpOnCheck1 false)
      (Variables|Default|SetJumpOnCheck2 false))))

(event Custom|RampJumped
  (bind _asbp_skater_player_state (Utilities|Casting|CastToBP_SkaterPlayerState (Variables|/Script/Engine.Pawn|GetPlayerState (Variables|Default|GetSkaterCharacter))))
  (Default|AddPoints _asbp_skater_player_state (Variables|Default|GetRampPoints)))

(fn ConstructionScript)